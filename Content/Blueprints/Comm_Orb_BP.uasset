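; Communication orb actor that floats ahead of and above player 0's pawn, trailing it with a bobbing motion.
; Each Tick it lerps toward the pawn-relative offset point by MovementRate, a per-frame alpha not scaled by delta time.
; Two timelines, with play rates set on BeginPlay, add vertical and horizontal bob along the pawn's up and right vectors after the lerp.
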(event EventBeginPlay
  ;[1 1 1] Start Bobbing
  (Components|Timeline|SetPlayRate (Variables|Default|GetHorizontalOffsetTimeline) (Variables|Default|GetHorizontalBobRate))
  (Components|Timeline|SetPlayRate (Variables|Default|GetVerticalOffsetTimeline) (Variables|Default|GetVerticalBobRate)))

(event EventTick
  (params (DeltaSeconds :type Float%20%28single-precision%29))
  (bind _returnvalue (Game|Player|GetPlayerPawn 0))
  (bind _returnvalue_2 (Transformation|GetActorUpVector _returnvalue))
  ;[1 1 1] Update Position
  (Transformation|SetActorLocation (+ (Math|Vector|Lerp(Vector) (Transformation|GetActorLocation) (+ (Transformation|GetActorLocation _returnvalue) (* (Transformation|GetActorForwardVector _returnvalue) (Variables|Default|GetForwardOffset)) (* _returnvalue_2 (Variables|Default|GetUpOffset))) (Variables|Default|GetMovementRate)) (* _returnvalue_2 (* (stale _offsettrack) (Variables|Default|GetVerticalBobDistance))) (* (Transformation|GetActorRightVector _returnvalue) (* (stale _offsettrack) (Variables|Default|GetHorizontalBobDistance)))) false false))

(fn ConstructionScript)