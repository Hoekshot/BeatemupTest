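; TestEnemy_BP is a test enemy that chases characters it sees and reacts to damage.
; PawnSensing sightings set InRange and start an AI MoveTo toward the seen character.
; Damage reduces Health, which starts at MaxHealth, and raises flinch flags while alive or death flags at zero.
; A disconnected branch holds unused movement logic for when nothing is in range, guarded by a Moving flag.
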(event `self.PawnSensing.OnSeePawn`
  (params (Pawn :type "Pawn Object Reference"))
  (set `self.In range` true)
  (bind _ascharacter (cast `Character` Pawn))
  (`|AIMoveTo` self (0.0 0.0 0.0) _ascharacter))

(event `self.ReceiveTick`
  (params (DeltaSeconds :type "Float (single-precision)")))

(event `self.ReceiveBeginPlay`
  (set `self.Health` (`self.MaxHealth`)))

(event `self.ReceiveAnyDamage`
  (params (Damage :type "Float (single-precision)") (DamageType :type "DamageType Object Reference") (InstigatedBy :type "Controller Object Reference") (DamageCauser :type "Actor Object Reference"))
  (if (not (`self.IsDead`))
    (bind _output_get (set `self.Health` (- (`self.Health`) Damage)))
    (if (> _output_get 0.0)
      (set `self.WillFlinch` true)
      (set `self.IsFlinching` true)
      (else
        (set `self.WillDie` true)
        (set `self.IsDead` true)))))

(fn `UserConstructionScript`)